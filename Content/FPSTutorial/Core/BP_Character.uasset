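; BP_Character is the player character for an FPS tutorial, driven by Enhanced Input through the IMC_FPS mapping context added on BeginPlay.
; Input actions move it along its forward and right vectors and turn the controller, with pitch inverted.
; Running raises max walk speed and plays a timeline that drives the camera manager's default FOV, then restores speed and reverses the timeline on release.
; A test action prints a debug string.
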(event `self.ReceiveBeginPlay`
  (`EnhancedInputSubsystemInterface.AddMappingContext` (pcsubsystem `EnhancedInputLocalPlayerSubsystem` (`GameplayStatics.GetPlayerController` 0)) "/Game/FPSTutorial/Data/IMC_FPS.IMC_FPS" 0 (struct)))

(event `EnhancedInput|/Game/FPSTutorial/Data/IA_Test`
  (params (ActionValue :type Boolean) (ElapsedSeconds :type "Float (double-precision)") (TriggeredSeconds :type "Float (double-precision)") (InputAction :type "InputAction Object Reference" :default "/Game/FPSTutorial/Data/IA_Test.IA_Test"))
  (:`Triggered`
    (`KismetSystemLibrary.PrintString` "TESTING")))

(event `EnhancedInput|/Game/FPSTutorial/Data/IA_Movement`
  (params (ActionValue :type "Vector2D Structure") (ElapsedSeconds :type "Float (double-precision)") (TriggeredSeconds :type "Float (double-precision)") (InputAction :type "InputAction Object Reference" :default "/Game/FPSTutorial/Data/IA_Movement.IA_Movement"))
  (bind (_x _y) (`KismetMathLibrary.BreakVector2D` ActionValue))
  (:`Triggered`
    (`self.AddMovementInput` (* (`self.GetActorForwardVector`) _y))
    (`self.AddMovementInput` (* (`self.GetActorRightVector`) _x))))

(event `EnhancedInput|/Game/FPSTutorial/Data/IA_Camera`
  (params (ActionValue :type "Vector2D Structure") (ElapsedSeconds :type "Float (double-precision)") (TriggeredSeconds :type "Float (double-precision)") (InputAction :type "InputAction Object Reference" :default "/Game/FPSTutorial/Data/IA_Camera.IA_Camera"))
  (bind (_x _y) (`KismetMathLibrary.BreakVector2D` ActionValue))
  (:`Triggered`
    ;[1 1 1] UP And Down
    (`self.AddControllerPitchInput` (* _y -1.0))
    (`self.AddControllerYawInput` _x) ; side ways
  ))

(event `EnhancedInput|/Game/FPSTutorial/Data/IA_Run`
  (params (ActionValue :type Boolean) (ElapsedSeconds :type "Float (double-precision)") (TriggeredSeconds :type "Float (double-precision)") (InputAction :type "InputAction Object Reference" :default "/Game/FPSTutorial/Data/IA_Run.IA_Run"))
  (:`Triggered`
    (set `CharacterMovementComponent.MaxWalkSpeed` 2000.0 (`self.CharacterMovement`))
    (bind (_direction _fov) (`Timeline|Timeline` :!label _label)
      (:`Update`
        (set `PlayerCameraManager.DefaultFOV` _fov (`GameplayStatics.GetPlayerCameraManager` 0)))))
  (:`Completed`
    (set `CharacterMovementComponent.MaxWalkSpeed` 600.0 (`self.CharacterMovement`))
    (goto _label :!via `Reverse`)))

(fn `UserConstructionScript`)